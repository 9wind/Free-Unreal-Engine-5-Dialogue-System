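; Talkable NPC that shows a name widget in range and, on interaction, hides and freezes the player to run a dialogue.
; Each DT_Dialogues row drives widget text, audio, montage, tag-selected camera and an overridable custom event.
; Rows chain on audio end or a fallback timer, pausing for decisions, with skip bound through the widget.
; An end-flagged row leads to restoring player, input and view, resetting to FirstTalk.
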(event `self.ReceiveBeginPlay`
  ;[1 1 1] Set Character Name
  (`/Game/Blueprints/WB_CharacterName.SetCharacterName` (`self.GetWidgetReference`) (`self.CharacterName`)))

(event `/Game/Blueprints/BPI_Interaction.EnterRange`
  ;[1 1 1] Widget/Interaction Management
  (`SceneComponent.SetVisibility` (`self.Widget`) true false)
  (set `self.AllowInteraction` true))

(event `/Game/Blueprints/BPI_Interaction.LeaveRange`
  ;[1 1 1] Widget/Interaction Management
  (`SceneComponent.SetVisibility` (`self.Widget`) false false)
  (set `self.AllowInteraction` false))

(event `/Game/Blueprints/BPI_Interaction.StartInteraction`
  (params (PlayerCharacter :type "Character Object Reference"))
  ;[1 1 1] Character Initialization
  (`self.Initializations` PlayerCharacter))

(event `StartMontage`
  (params (MontageToPlay :type "AnimMontage Object Reference"))
  (bind _mesh (`self.Mesh`))
  (bind _returnvalue (`SkeletalMeshComponent.GetAnimInstance` _mesh))
  ;[1 1 1] Play Montage
  (`/Engine/EditorBlueprintResources/StandardMacros.IsValid` MontageToPlay
    (:`Is Valid`
      (if (not (`AnimInstance.IsAnyMontagePlaying` _returnvalue))
        (`AnimInstance.Montage_Stop` _returnvalue 0.25 (`AnimInstance.GetCurrentActiveMontage` _returnvalue))
        (`KismetSystemLibrary.Delay` 0.25))
      (`|PlayMontage` _mesh MontageToPlay))))

(fn `EndInteraction`
  (bind _returnvalue (`GameplayStatics.GetPlayerController` 0))
  ;[0.05098 0.05098 0.05098 1 40] End Interaction, shows player, switches game mode and allow player to do previous state
  ;;[0.9683 0.5248 1] here we can set another additional index
  (set `self.CurrentDialogueIndex` "FirstTalk")
  (set `self.EndDial` false)
  (`self.SetActorHiddenInGame` (`self.Player Character`) false)
  (`Widget.RemoveFromParent` (`self.WidgetInterface`))
  (`CharacterMovementComponent.SetMovementMode` (`Character.CharacterMovement` (`self.Player Character`)) "MOVE_Walking" 0)
  (`WidgetBlueprintLibrary.SetInputMode_GameOnly` _returnvalue)
  (set `PlayerController.bShowMouseCursor` false _returnvalue)
  (`PlayerController.SetViewTargetWithBlend` _returnvalue (`GameplayStatics.GetPlayerPawn` 0) 0.0 "VTBlend_Linear" 0.0 false))

(fn `FireCustomEvent`
  (bind ((`CustomEvent_32_FC92B9734146B30E77FAFC9C95712ACC` _customevent)) (break `/Game/Blueprints/ST_Dialogue` (`self.GetDataTableRowIndex` (`self.CurrentDialogueIndex`))))
  ;[0.05098 0.05098 0.05098] Overwrite this function for your custom events!
  (if (not (`KismetStringLibrary.IsEmpty` _customevent))
    (bind _returnvalue (`GameplayStatics.GetActorOfClass` "/Game/Blueprints/SM_ChamferCube2.SM_ChamferCube2_C"))
    (`/Game/Blueprints/SM_ChamferCube2.SetColor` _returnvalue _customevent)))

(fn `GetCameraTag`
  (params (Tag :type Name))
  (returns (CameraRef :type "/Game/Blueprints/DialogueCamera Object Reference"))
  ;[0.05098 0.05098 0.05098 1 30] Get Camera Tag That will be blend in
  (bind _outactors (`GameplayStatics.GetAllActorsOfClassWithTag` "/Game/Blueprints/DialogueCamera.DialogueCamera_C" Tag))
  (if (`KismetArrayLibrary.Array_IsValidIndex` _outactors)
    (return (`|GetArrayItem` _outactors))
    (else
      (`KismetSystemLibrary.PrintString` "Wrong Camera Index")
      (return null))))

(fn `GetDataTableRowIndex`
  (params (RowName :type Name))
  (returns (`Out Row` :type "/Game/Blueprints/ST_Dialogue Structure"))
  ;[0.05098 0.05098 0.05098 1 40] Get DataTable Row Dialogue Details
  (bind _returnvalue (`|GetDataTableRow` "/Game/Blueprints/DT_Dialogues.DT_Dialogues" RowName)
    (:`then`
      (return _returnvalue))))

(fn `GetWidgetReference`
  (returns (WidgetReference :type "/Game/Blueprints/WB_CharacterName Object Reference"))
  ;[0.05098 0.05098 0.05098] Get Widget Reference that is attached to character and displays name for example
  (bind _aswb_character_name (cast `/Game/Blueprints/WB_CharacterName` (`WidgetComponent.GetWidget` (`self.Widget`)))
    (:`then`
      (return _aswb_character_name))
    (:`CastFailed`
      (`KismetSystemLibrary.PrintString` "wrong widget"))))

(fn `Initializations`
  (params (`Player Character` :type "Character Object Reference"))
  (bind _returnvalue (`GameplayStatics.GetPlayerController` 0))
  (bind _widgetinterface (`self.WidgetInterface`))
  (bind _charactermovement (`Character.CharacterMovement` (`self.Player Character`)))
  ;[0.05098 0.05098 0.05098 1 30] Dialogue Initialization - stops movement, hides player and name widget, show dialogue widget and switches game mode
  (if (`self.AllowInteraction`)
    (set `self.Player Character` `Player Character`)
    (set `self.AllowInteraction` false)
    (`MovementComponent.StopMovementImmediately` _charactermovement)
    (`CharacterMovementComponent.DisableMovement` _charactermovement)
    (`self.SetActorHiddenInGame` (`self.Player Character`) true)
    (`SceneComponent.SetVisibility` (`self.Widget`) false false)
    (bind _returnvalue_2 (`|CreateWidget` "/Game/Blueprints/WB_MainDialogueWidget.WB_MainDialogueWidget_C" null self))
    (bind _output_get (set `self.WidgetInterface` _returnvalue_2))
    (`UserWidget.AddToViewport` _output_get 0)
    (`WidgetBlueprintLibrary.SetInputMode_GameAndUIEx` _returnvalue _returnvalue_2)
    (set `PlayerController.bShowMouseCursor` true _returnvalue)
    ;;[1 0.8908 0.3944] space - skip
    (add `/Game/Blueprints/WB_MainDialogueWidget.Skip` _widgetinterface (`|CreateDelegate` :!event `PlayDialogue`))
    (`/Game/Blueprints/WB_MainDialogueWidget.SetTextInitialAnim` _widgetinterface (`.Text_4_B44670014BC99944A0CA94B7FC468C4E` (break `/Game/Blueprints/ST_Dialogue` (`self.GetDataTableRowIndex` (`self.CurrentDialogueIndex`)))))
    (`self.PlayDialogue`)))

(fn `PlayDialogue`
  (bind _audio (`self.Audio`))
  (bind (_out_row_text _out_row_audio _out_row_montage _out_row_customcamera_ _out_row_nextdialogue _out_row_decisions _out_row_shouldend_) (break `/Game/Blueprints/ST_Dialogue` (`self.GetDataTableRowIndex` (`self.CurrentDialogueIndex`))))
  (bind _cameraref (`self.GetCameraTag` _out_row_customcamera_))
  (`KismetSystemLibrary.K2_ClearTimer` null "PlayDialogue") ; prevents doublepicking when no audio available
  (if (`self.EndDial`)
    (`self.EndInteraction`)
    (else
      (`/Game/Blueprints/WB_MainDialogueWidget.PlayAnotherTextAnimation` (`self.WidgetInterface`) _out_row_text)
      (set `self.EndDial` _out_row_shouldend_)
      (`self.FireCustomEvent`)
      (`/Engine/EditorBlueprintResources/StandardMacros.IsValid` _out_row_audio
        (:`Is Valid`
          (`AudioComponent.SetSound` _audio _out_row_audio)
          (`AudioComponent.Play` _audio 0.0))
        (:`Is Not Valid`
          _))
      (`self.StartMontage` _out_row_montage)
      (`/Engine/EditorBlueprintResources/StandardMacros.IsValid` _cameraref
        (:`Is Valid`
          (`PlayerController.SetViewTargetWithBlend` (`GameplayStatics.GetPlayerController` 0) _cameraref 0.0 "VTBlend_Linear" 0.0 false))
        (:`Is Not Valid`
          _))
      (if (`KismetArrayLibrary.Array_IsValidIndex` _out_row_decisions)
        ;[1 1 1] Populate Decision
        (`/Game/Blueprints/WB_MainDialogueWidget.AddDecisions` (`self.WidgetInterface`) _out_row_decisions)
        (else
          (`/Engine/EditorBlueprintResources/StandardMacros.IsValid` _out_row_audio
            (:`Is Valid`
              (add `AudioComponent.OnAudioFinished` (`self.Audio`) (`|CreateDelegate` :!event `PlayDialogue`)))
            (:`Is Not Valid`
              (`KismetSystemLibrary.K2_SetTimer` null "PlayDialogue" 3.0) ; default time if audio is invalid
            ))
          ;[1 1 1] Set Next Dial if not decision
          (set `self.CurrentDialogueIndex` (`.NextDialogue_24_BFE61BBA4D116466BDAA6A9812CDB285` (break `/Game/Blueprints/ST_Dialogue` (`self.GetDataTableRowIndex` (`self.CurrentDialogueIndex`))))))))))

(fn `UserConstructionScript`)